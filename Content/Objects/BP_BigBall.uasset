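; BP_BigBall is a heavy ball that triggers gate flags when it reaches tagged plates.
; On BeginPlay it scales its Sphere's mass by MassScaleMultiplier.
; Overlapping a BP_Plate tagged GateOne or GateTwo sets the matching gate to true on its parent actor, Test_DemoLogic, so it relies on being that actor's child.
; Nothing here resets a gate when the ball leaves.
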(event EventBeginPlay
  (Class|PrimitiveComponent|SetMassScale (Variables|Default|GetSphere) "None" (Variables|Default|GetMassScaleMultiplier)))

(event Collision|EventActorBeginOverlap
  (params (OtherActor :type Actor%20Object%20Reference))
  (bind _returnvalue (Actor|GetParentActor))
  (bind _asbp_plate (Utilities|Casting|CastToBP_Plate OtherActor))
  (if (Actor|ActorHasTag _asbp_plate "GateOne")
    (bind _astest_demo_logic (Utilities|Casting|CastToTest_DemoLogic _returnvalue))
    (Default|SetGateOne _astest_demo_logic true)
    (elif (Actor|ActorHasTag _asbp_plate "GateTwo")
      (bind _astest_demo_logic_2 (Utilities|Casting|CastToTest_DemoLogic _returnvalue))
      (Default|SetGateTwo _astest_demo_logic_2 true))))

(fn ConstructionScript)