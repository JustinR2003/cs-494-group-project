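; Pressure plate puzzle Blueprint that is solved when a pushable cube overlaps the activate box without touching the deactivate box.
; Tick polls both overlaps and swaps each box's monitor material as feedback until PuzzleDone is set.
; Once solved, a DoOnce plays a timeline that animates the cube's scale, then destroys the cube component.
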(event EventTick
  (params (DeltaSeconds :type Float%20%28single-precision%29))
  (bind _deactivatebox (Variables|Default|GetDeactivateBox))
  (bind _pushable_cube (Variables|Default|GetPushable%20Cube))
  (bind _returnvalue (Class|PrimitiveComponent|IsOverlappingComponent _pushable_cube _deactivatebox))
  (if (Variables|Default|GetPuzzleDone)
    (Utilities|FlowControl|DoOnce false
      (:Completed
        (bind _newtrack_0 (Timeline|Timeline Play)
          (:Update
            (Transformation|SetRelativeScale3D (Variables|Default|GetPushable%20Cube) (Math|Conversions|ToVector(Float) _newtrack_0)))
          (:Finished
            (Components|DestroyComponent (Variables|Default|GetPushable%20Cube))))))
    (else
      (Utilities|FlowControl|Sequence
        (:then_0
          (if _returnvalue
            (Rendering|Material|SetMaterial (Variables|Default|GetMonitor_r2) 1 "/Game/MyMaterials/Blue.Blue")
            (else
              (Rendering|Material|SetMaterial (Variables|Default|GetMonitor_r2) 1 "/Game/CRT_VCR_Material/Materials/T_Trace/Background_material.Background_material"))))
        (:then_1
          (if (Class|PrimitiveComponent|IsOverlappingComponent (Variables|Default|GetPushable%20Cube) (Variables|Default|GetActivateBox))
            (Rendering|Material|SetMaterial (Variables|Default|GetMonitor_r1) 1 "/Game/CRT_VCR_Material/Materials/Presets/CRT_Preset_320x224.CRT_Preset_320x224")
            (if (not _returnvalue)
              (Variables|Default|SetPuzzleDone true))
            (else
              (Rendering|Material|SetMaterial (Variables|Default|GetMonitor_r1) 1 "/Game/CRT_VCR_Material/Materials/T_Trace/Background_material.Background_material"))))))))

(fn ConstructionScript)