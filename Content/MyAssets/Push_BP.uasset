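; Push_BP is a puzzle Blueprint that tracks two monitors, NonworkingMonitor and WorkingMonitor, by their world X position.
; Every Tick, it compares each monitor against its own fixed X threshold and swaps that monitor's screen material accordingly.
; It also sets PuzzleDone each frame, true only while both monitors are past their thresholds in opposite directions, so the solved state is not latched.
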(event EventTick
  (params (DeltaSeconds :type Float%20%28single-precision%29))
  (bind _workingmonitor (Variables|Default|GetworkingMonitor))
  (bind _nonworkingmonitor (Variables|Default|GetnonworkingMonitor))
  (bind _nonworkingmonitor_2 (Variables|Default|GetnonworkingMonitor))
  (bind _workingmonitor_2 (Variables|Default|GetworkingMonitor))
  (bind _returnvalue (Transformation|GetWorldLocation _nonworkingmonitor))
  (bind _returnvalue_2 (Transformation|GetWorldLocation _workingmonitor))
  (bind _returnvalue_3 (> (.x _returnvalue) 425.0))
  (bind _returnvalue_4 (< (.x _returnvalue_2) -4.5e+02))
  (Utilities|FlowControl|Sequence
    (:then_0
      (if _returnvalue_3
        (Rendering|Material|SetMaterial _nonworkingmonitor_2 1 "/Game/CRT_VCR_Material/Meshes/TV_Materials/TV_black.TV_black")
        (else
          (Rendering|Material|SetMaterial _nonworkingmonitor_2 1 "/Game/MyMaterials/Blue.Blue"))))
    (:then_1
      (if _returnvalue_4
        (Rendering|Material|SetMaterial _workingmonitor_2 1 "/Game/CRT_VCR_Material/Materials/00_animated_crt_v2_1.00_animated_crt_v2_1")
        (else
          (Rendering|Material|SetMaterial _workingmonitor_2 1 "/Game/CRT_VCR_Material/Materials/Presets/CRT_Preset_640x480.CRT_Preset_640x480"))))
    (:then_2
      (Variables|Default|SetPuzzleDone (and _returnvalue_3 _returnvalue_4)))))

(fn ConstructionScript)