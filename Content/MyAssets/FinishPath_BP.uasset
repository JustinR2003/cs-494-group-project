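; FinishPath_BP is an actor for a finish path that stays hidden until the level's puzzle is complete, then animates into view.
; Every Tick it looks up PuzzleComplete_BP and checks LevelComplete, zeroing the mesh scale once while incomplete.
; Once complete, a one-shot delay of a few seconds starts two timelines that drive the mesh's relative scale and X location together.
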(event EventTick
  (params (DeltaSeconds :type Float%20%28single-precision%29))
  (bind _returnvalue (Actor|GetActorOfClass "/Game/MyAssets/PuzzleComplete_BP.PuzzleComplete_BP_C"))
  (if (Variables|/Game/MyAssets/PuzzleComplete_BP.PuzzleComplete_BP_C|GetLevelComplete _returnvalue)
    (Utilities|FlowControl|DoOnce false
      (:Completed
        (Utilities|FlowControl|Delay 5.0)
        (Utilities|FlowControl|Sequence
          (:then_0
            (bind _newtrack_1 (Timeline|Timeline Play)
              (:Update
                (Transformation|SetRelativeScale3D (Variables|Debug|GetStaticMeshComponent) _newtrack_1))))
          (:then_1
            (bind _newtrack_0 (Timeline|Timeline_0 Play)
              (:Update
                (Transformation|SetRelativeLocation (Variables|Debug|GetStaticMeshComponent) (Math|Vector|MakeVector _newtrack_0 0.0 0.0) false false)))))))
    (else
      (Utilities|FlowControl|DoOnce false
        (:Completed
          (Transformation|SetRelativeScale3D (Variables|Debug|GetStaticMeshComponent) "0, 0, 0"))))))

(fn ConstructionScript)