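; Maze actor that moves vertically once two ComputerInteract_Blueprint computers are activated, as part of a puzzle.
; Tick fetches all computer actors every frame and checks the Activated flag on the first two.
; A DoOnce then plays a timeline that adds its MoveDown value to the actor's current Z on each update, so movement accumulates, and sets PuzzleDone when finished.
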(event EventTick
  (params (DeltaSeconds :type Float%20%28single-precision%29))
  (bind _returnvalue (Transformation|GetActorLocation))
  (bind (_x _y _z) (Math|Vector|BreakVector _returnvalue))
  (bind _outactors (Actor|GetAllActorsOfClass "/Game/MyAssets/ComputerInteract_Blueprint.ComputerInteract_Blueprint_C"))
  (if (and (Variables|/Game/MyAssets/ComputerInteract_Blueprint.ComputerInteract_Blueprint_C|GetActivated (Utilities|Array|Get(acopy) _outactors)) (Variables|/Game/MyAssets/ComputerInteract_Blueprint.ComputerInteract_Blueprint_C|GetActivated (Utilities|Array|Get(acopy) _outactors 1)))
    (Utilities|FlowControl|DoOnce false
      (:Completed
        (bind _movedown (Timeline|Timeline Play)
          (:Update
            (Transformation|SetActorLocation (Math|Vector|MakeVector _x _y (+ _z _movedown)) false false))
          (:Finished
            (Variables|Default|SetPuzzleDone true)))))))

(fn ConstructionScript)