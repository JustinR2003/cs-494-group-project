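; PuzzleComplete_BP is an actor that decides when the level is complete, based on three puzzles and the player's position.
; Each Tick until completion, it looks up one Maze_BP, Push_BP and PressurePlate_BP through GetActorOfClass and reads their PuzzleDone flags.
; LevelComplete becomes true when all three flags are set while the player character overlaps this actor, which stops further checks.
; It only sets that flag and triggers nothing else itself.
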(event EventTick
  (params (DeltaSeconds :type Float%20%28single-precision%29))
  (if (not (Variables|Default|GetLevelComplete))
    (Utilities|FlowControl|Sequence
      (:then_0
        (bind _returnvalue (Actor|GetActorOfClass "/Game/MyAssets/Maze_BP.Maze_BP_C")))
      (:then_1
        (bind _returnvalue_2 (Actor|GetActorOfClass "/Game/MyAssets/Push_BP.Push_BP_C")))
      (:then_2
        (bind _returnvalue_3 (Actor|GetActorOfClass "/Game/MyAssets/PressurePlate_BP.PressurePlate_BP_C")))
      (:then_3
        (Variables|Default|SetLevelComplete (and (and (and (Variables|/Game/MyAssets/Maze_BP.Maze_BP_C|GetPuzzleDone _returnvalue) (Variables|/Game/MyAssets/Push_BP.Push_BP_C|GetPuzzleDone _returnvalue_2)) (Variables|/Game/MyAssets/PressurePlate_BP.PressurePlate_BP_C|GetPuzzleDone _returnvalue_3)) (Collision|IsOverlappingActor (Game|GetPlayerCharacter 0) :!class /Script/Engine.Actor)))))))

(fn ConstructionScript)