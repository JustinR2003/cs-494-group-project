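; LowerMonitors_BP is an actor that moves vertically, by its name lowering monitors, once the Push_BP puzzle is done.
; Every Tick until solved, it looks up the Push_BP actor and plays a timeline when PuzzleDone is true.
; Each timeline update adds MoveDown to the current Z, so movement accumulates per frame rather than interpolating between fixed positions.
; When the timeline finishes, Solved stops further checks.
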(event EventTick
  (params (DeltaSeconds :type Float%20%28single-precision%29))
  (bind _returnvalue (Transformation|GetActorLocation))
  (bind (_x _y _z) (Math|Vector|BreakVector _returnvalue))
  (if (not (Variables|Default|GetSolved))
    (bind _returnvalue_2 (Actor|GetActorOfClass "/Game/MyAssets/Push_BP.Push_BP_C"))
    (if (Variables|/Game/MyAssets/Push_BP.Push_BP_C|GetPuzzleDone _returnvalue_2)
      (bind _movedown (Timeline|Timeline Play)
        (:Update
          (Transformation|SetActorLocation (Math|Vector|MakeVector _x _y (+ _z _movedown)) false false))
        (:Finished
          (Variables|Default|SetSolved true))))))

(fn ConstructionScript)